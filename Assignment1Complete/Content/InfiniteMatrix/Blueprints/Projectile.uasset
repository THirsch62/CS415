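; Projectile actor that flies along world X and kills enemies on contact.
; Tick advances its X location by Speed times delta time, and SetSpeed stores the supplied speed scaled by a fixed multiplier.
; Any sphere overlap destroys the projectile; if the other actor is an Enemy, it is destroyed too and the player pawn's BP_Player score increases.
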(event OnComponentBeginOverlap(Sphere)
  (params (OverlappedComponent :type Primitive%20Component%20Object%20Reference) (OtherActor :type Actor%20Object%20Reference) (OtherComp :type Primitive%20Component%20Object%20Reference) (OtherBodyIndex :type Integer) (bFromSweep :type Boolean) (SweepResult :type Hit%20Result%20Structure%20%28by%20ref%29))
  (Actor|DestroyActor)
  (bind _asenemy (Utilities|Casting|CastToEnemy OtherActor))
  (Actor|DestroyActor _asenemy)
  (bind _asbp_player (Utilities|Casting|CastToBP_Player (Game|Player|GetPlayerPawn 0)))
  (Default|UpdateScore _asbp_player 5))

(event EventBeginPlay)

(event Collision|EventActorBeginOverlap
  (params (OtherActor :type Actor%20Object%20Reference)))

(event EventTick
  (params (DeltaSeconds :type Float%20%28single-precision%29))
  (bind _returnvalue (Transformation|GetActorLocation))
  (Transformation|SetActorLocation (Math|Vector|MakeVector (+ (* DeltaSeconds (Variables|Default|GetSpeed)) (.x _returnvalue)) (.y _returnvalue) (.z _returnvalue)) false false))

(fn ConstructionScript)

(fn SetSpeed
  (params (Speed :type Float%20%28double-precision%29))
  (Variables|Default|SetSpeed (* Speed 1.5)))